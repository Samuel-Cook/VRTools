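; BP_ShotgunShell is a shotgun round for the VR gun toolkit that loads directly into the gun rather than into a magazine.
; While held, overlapping a gun's MagazineTrigger adds its class to that gun's non-full ammo array, plays a sound and destroys the actor.
; As a bullet, it spawns multiple shrapnel actors with random rotational spread.
; As a fired casing, it swaps to an exploded mesh and drops its trigger box.
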(event `self.Box.OnComponentBeginOverlap`
  (params (OverlappedComponent :type "PrimitiveComponent Object Reference") (OtherActor :type "Actor Object Reference") (OtherComp :type "PrimitiveComponent Object Reference") (OtherBodyIndex :type Integer) (bFromSweep :type Boolean) (SweepResult :type "HitResult Structure (by ref)"))
  ;[0.5357 1 0.3115] Load this ammo directly to the Gun instead of Magazine
  (if (`self.HeldInHand`)
    (bind _asbp_vrrealistic_gun_base (cast `/Game/VRGunToolkit/Blueprints/BP_VRRealisticGun_Base` OtherActor)
      (:`then`
        (bind _magazine (`/Game/VRGunToolkit/Blueprints/BP_VRRealisticGun_Base.Magazine` _asbp_vrrealistic_gun_base))
        (bind _ammo (`/Game/VRGunToolkit/Blueprints/BP_VRRealisticMagazine.Ammo` _magazine))
        (if (and (== OtherComp (`/Game/VRGunToolkit/Blueprints/BP_VRRealisticGun_Base.MagazineTrigger` _asbp_vrrealistic_gun_base)) (< (`KismetArrayLibrary.Array_Length` _ammo) (`/Game/VRGunToolkit/Blueprints/BP_VRRealisticMagazine.MaxAmmo` _magazine)))
          (`GameplayStatics.PlaySoundAtLocation` "/Game/VRGunToolkit/Sounds/Pistol/Wav/A_Pistol_SlideBack.A_Pistol_SlideBack" (`self.K2_GetActorLocation`))
          (`KismetArrayLibrary.Array_Add` _ammo (`GameplayStatics.GetObjectClass` self))
          (`self.K2_DestroyActor`)))
      (:`CastFailed`
        (`KismetSystemLibrary.PrintString` "Failed cast to the Gun on BeginOverlap" false true (struct :`R` 1.0 :`B` 0.009947 :`A` 1.0) 5.0)))))

(event `self.BulletOnly`
  ;[0.6607 1 0.5015] Shotgun bullet spread
  (`ActorComponent.K2_DestroyComponent` (`self.Box`))
  (`parent.BulletOnly`)
  (for _ (range 11)
    (bind _returnvalue (`|SpawnActorFromClass` "/Game/VRGunToolkit/Blueprints/Projectiles/Shell/BP_ShotGunShrapnel.BP_ShotGunShrapnel_C" (`KismetMathLibrary.MakeTransform` (`self.K2_GetActorLocation`) (`KismetMathLibrary.ComposeRotators` (`KismetMathLibrary.MakeRotator` (`KismetMathLibrary.RandomFloatInRange` -5.0 5.0) (`KismetMathLibrary.RandomFloatInRange` -5.0 5.0) (`KismetMathLibrary.RandomFloatInRange` -5.0 5.0)) (`self.K2_GetActorRotation`))) "AlwaysSpawn" "OverrideRootScale"))
    (`self.BulletOnly` _returnvalue)))

(event `self.ShellOnly`
  (params (Fired :type Boolean))
  ;[1 0.6914 0.4222] Set Mesh of the Shell to the "exploded" one if we fired
  (`parent.ShellOnly` Fired)
  (if Fired
    (`StaticMeshComponent.SetStaticMesh` (`self.Shell`) "/Game/VRGunToolkit/Meshes/Weapons/Bullet/SM_ShotgunShellExploded.SM_ShotgunShellExploded")
    (`ActorComponent.K2_DestroyComponent` (`self.Box`))))

(fn `UserConstructionScript`
  (`parent.UserConstructionScript`))