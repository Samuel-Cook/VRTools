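; Shooting range target for the VR gun toolkit demo room, with events to step it forward or backward and to reset it.
; Each step shifts the target mesh along world X by the X offset found 100 units along the spline, staying between the first two spline points.
; Reset destroys the mesh's child components, such as decals, but spares point lights, repeating until at most one child remains.
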(event `Forward`
  (bind _spline (`self.Spline`))
  (bind (_returnvalue_x _returnvalue_y _returnvalue_z) (`KismetMathLibrary.BreakVector` (`SceneComponent.K2_GetComponentLocation` (`self.TargetMesh`))))
  (bind _returnvalue_x_2 (`KismetMathLibrary.BreakVector` (`SplineComponent.GetLocationAtDistanceAlongSpline` _spline 100.0 "Local")))
  (bind _returnvalue_x_3 (`KismetMathLibrary.BreakVector` (`SplineComponent.GetLocationAtSplinePoint` _spline 1 "World")))
  (bind _returnvalue (+ _returnvalue_x _returnvalue_x_2))
  ;[1 1 1] Go Forward
  (if (> _returnvalue_x_3 _returnvalue)
    (`SceneComponent.K2_SetWorldLocation` (`self.TargetMesh`) (`KismetMathLibrary.MakeVector` _returnvalue _returnvalue_y _returnvalue_z) false false)))

(event `Backward`
  (bind _spline (`self.Spline`))
  (bind _returnvalue_x (`KismetMathLibrary.BreakVector` (`SplineComponent.GetLocationAtDistanceAlongSpline` _spline 100.0 "Local")))
  (bind _returnvalue_x_2 (`KismetMathLibrary.BreakVector` (`SplineComponent.GetLocationAtSplinePoint` _spline 0 "World")))
  (bind (_returnvalue_x_3 _returnvalue_y _returnvalue_z) (`KismetMathLibrary.BreakVector` (`SceneComponent.K2_GetComponentLocation` (`self.TargetMesh`))))
  (bind _returnvalue (- _returnvalue_x_3 _returnvalue_x))
  ;[1 1 1] Go Backward
  (if (< _returnvalue_x_2 _returnvalue)
    (`SceneComponent.K2_SetWorldLocation` (`self.TargetMesh`) (`KismetMathLibrary.MakeVector` _returnvalue _returnvalue_y _returnvalue_z) false false)))

(event `Reset_Target`
  (bind _returnvalue (`SceneComponent.GetNumChildrenComponents` (`self.TargetMesh`)))
  ;[1 1 1] Remove Decals on Target
  (`/Engine/EditorBlueprintResources/StandardMacros.DoOnce` false :!label _label
    (:`Completed`
      (for _index (range (+ _returnvalue 1)) :!label _label_2
        (bind _returnvalue_2 (`SceneComponent.GetChildComponent` (`self.TargetMesh`) _index))
        (cast `PointLightComponent` _returnvalue_2 ; Avoid to destroy the light attached
          (:`CastFailed`
            (`ActorComponent.K2_DestroyComponent` _returnvalue_2) ; Destroy decals
          )))
      (if (> _returnvalue 1)
        (goto _label_2)
        (else
          (goto _label :!via `Reset`))))))

(fn `UserConstructionScript`)