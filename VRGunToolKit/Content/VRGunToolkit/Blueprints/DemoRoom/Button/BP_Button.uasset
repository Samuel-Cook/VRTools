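; BP_Button is a physical push button in the VR gun toolkit demo room that moves a BP_MovingTarget forward, backward or resets it.
; An overlapping component's travel along the button's local Z sets a clamped press depth, and the button eases back when released.
; A full press fires the action for its type on the first target found, with a DoOnce re-armed after a short delay, longer for reset.
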(event `self.ReceiveBeginPlay`
  (set `self.Init_Location` (`SceneComponent.RelativeLocation` (`self.BTN`)))
  (bind _outactors (`GameplayStatics.GetAllActorsOfClass` "/Game/VRGunToolkit/Blueprints/DemoRoom/BP_MovingTarget.BP_MovingTarget_C"))
  (set `self.TargetReference` (`KismetArrayLibrary.Array_Get` _outactors)))

(event `self.ReceiveTick`
  (params (DeltaSeconds :type "Float (single-precision)"))
  (bind _btn (`self.BTN`))
  (bind _targetreference (`self.TargetReference`))
  (bind (_returnvalue_x _returnvalue_y _returnvalue_z) (`KismetMathLibrary.BreakVector` (- (`KismetMathLibrary.InverseTransformDirection` (`SceneComponent.K2_GetComponentToWorld` _btn) (`self.Start Location`)) (`KismetMathLibrary.InverseTransformDirection` (`SceneComponent.K2_GetComponentToWorld` _btn) (`SceneComponent.K2_GetComponentLocation` (`self.Overlap`))))))
  (bind _returnvalue (`KismetMathLibrary.FClamp` _returnvalue_z 0.0 (`self.MaxButtonPress`)))
  (`/Engine/EditorBlueprintResources/StandardMacros.IsValid` (`self.Overlap`)
    (:`Is Valid`
      (set `self.ButtonPressAmount` _returnvalue)
      (`SceneComponent.K2_SetRelativeLocation` (`self.BTN`) (- (`self.Init_Location`) (`KismetMathLibrary.MakeVector` 0.0 0.0 _returnvalue)) false false)
      (if (>= (`self.ButtonPressAmount`) (`self.MaxButtonPress`))
        (`/Engine/EditorBlueprintResources/StandardMacros.DoOnce` false :!label _label
          (:`Completed`
            (switch `/Game/VRGunToolkit/Blueprints/DemoRoom/Button/ENUM_BTN_State` (`self.TypeOfBTN`)
              (:`NewEnumerator0`
                (`/Game/VRGunToolkit/Blueprints/DemoRoom/BP_MovingTarget.Forward` _targetreference)
                (`KismetSystemLibrary.Delay` 0.08 :!label _label_2))
              (:`NewEnumerator1`
                (`/Game/VRGunToolkit/Blueprints/DemoRoom/BP_MovingTarget.Backward` _targetreference)
                (goto _label_2))
              (:`NewEnumerator2`
                (`/Game/VRGunToolkit/Blueprints/DemoRoom/BP_MovingTarget.Reset_Target` _targetreference)
                (`KismetSystemLibrary.Delay` 2.0)))
            (`self.Reset`)))))
    (:`Is Not Valid`
      (`SceneComponent.K2_SetRelativeLocation` (`self.BTN`) (`KismetMathLibrary.VInterpTo` (`SceneComponent.RelativeLocation` (`self.BTN`)) (`self.Init_Location`) DeltaSeconds 8.0) false false))))

(event `Reset`
  (goto _label :!via `Reset`))

(event `self.BTN.OnComponentBeginOverlap`
  (params (OverlappedComponent :type "PrimitiveComponent Object Reference") (OtherActor :type "Actor Object Reference") (OtherComp :type "PrimitiveComponent Object Reference") (OtherBodyIndex :type Integer) (bFromSweep :type Boolean) (SweepResult :type "HitResult Structure (by ref)"))
  (`/Engine/EditorBlueprintResources/StandardMacros.IsValid` (`self.Overlap`)
    (:`Is Not Valid`
      (bind _output_get (set `self.Overlap` OtherComp))
      (set `self.Start Location` (`SceneComponent.K2_GetComponentLocation` _output_get)))))

(event `self.BTN.OnComponentEndOverlap`
  (params (OverlappedComponent :type "PrimitiveComponent Object Reference") (OtherActor :type "Actor Object Reference") (OtherComp :type "PrimitiveComponent Object Reference") (OtherBodyIndex :type Integer))
  (if (== OtherComp (`self.Overlap`))
    (set `self.Overlap` null)))

(fn `UserConstructionScript`
  (`TextRenderComponent.K2_SetText` (`self.TextRender`) (`self.BTN_TXT`)))