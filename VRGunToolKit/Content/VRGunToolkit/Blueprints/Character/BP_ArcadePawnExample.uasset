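; Example arcade VR pawn that carries two hip holsters and automatically refills them with Colt 1911 pistols.
; Every Tick places both holsters below and beside the camera, following only its yaw with a fixed downward pitch.
; A holster with no child components starts its own timer, guarded by handle validity, which after a short delay spawns and attaches a BP_Colt1911_Arcade, then clears the handle.
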(event `self.ReceiveBeginPlay`
  ;[1 1 1] BeginPlay
  (`parent.ReceiveBeginPlay`))

(event `Create Right Gun`
  ;[0.1419 1 0.1864] Spawn Guns on our hips
  (`self.SpawnGunInHolster` (`self.HolsterRight`))
  (`KismetSystemLibrary.K2_ClearAndInvalidateTimerHandle` (`self.TimerRight`)))

(event `self.ReceiveTick`
  (params (DeltaSeconds :type "Float (single-precision)"))
  (bind _camera (`self.Camera`))
  (bind (_returnvalue_roll _returnvalue_pitch _returnvalue_yaw) (`KismetMathLibrary.BreakRotator` (`SceneComponent.K2_GetComponentRotation` _camera)))
  (bind _relativelocation (`SceneComponent.RelativeLocation` (`self.Camera`)))
  (bind (_returnvalue_roll_2 _returnvalue_pitch_2 _returnvalue_yaw_2) (`KismetMathLibrary.BreakRotator` (`KismetMathLibrary.ComposeRotators` (`SceneComponent.RelativeRotation` _camera))))
  ;[0.1765 0.2409 1] Tick, Set holster Position and activate timers when we take out one of the guns
  (`SceneComponent.K2_SetRelativeLocation` (`self.HolsterRight`) (- _relativelocation (`KismetMathLibrary.GreaterGreater_VectorRotator` (0.0 20.0 60.0) (`KismetMathLibrary.MakeRotator` 0.0 0.0 _returnvalue_yaw_2))) false false)
  (`SceneComponent.K2_SetRelativeLocation` (`self.HolsterLeft`) (- _relativelocation (`KismetMathLibrary.GreaterGreater_VectorRotator` (0.0 -20.0 60.0) (`KismetMathLibrary.MakeRotator` 0.0 0.0 _returnvalue_yaw_2))) false false)
  (`SceneComponent.K2_SetWorldRotation` (`self.HolsterLeft`) (`KismetMathLibrary.MakeRotator` 0.0 -45.0 _returnvalue_yaw) false false)
  (`SceneComponent.K2_SetWorldRotation` (`self.HolsterRight`) (`KismetMathLibrary.MakeRotator` 0.0 -45.0 _returnvalue_yaw) false false)
  (`|ExecutionSequence`
    (:`then_0`
      (if (and (== (`SceneComponent.GetNumChildrenComponents` (`self.HolsterRight`)) 0) (not (`KismetSystemLibrary.K2_IsValidTimerHandle` (`self.TimerRight`))))
        (bind _returnvalue (`KismetSystemLibrary.K2_SetTimer` null "Create Right Gun" 5.0))
        (set `self.TimerRight` _returnvalue)))
    (:`then_1`
      (if (and (== (`SceneComponent.GetNumChildrenComponents` (`self.HolsterLeft`)) 0) (not (`KismetSystemLibrary.K2_IsValidTimerHandle` (`self.TimerLeft`))))
        (bind _returnvalue_2 (`KismetSystemLibrary.K2_SetTimer` null "Create Left Gun" 5.0))
        (set `self.TimerLeft` _returnvalue_2)))))

(event `Create Left Gun`
  ;[0.1419 1 0.1864] Spawn Guns on our hips
  (`self.SpawnGunInHolster` (`self.HolsterLeft`))
  (`KismetSystemLibrary.K2_ClearAndInvalidateTimerHandle` (`self.TimerLeft`)))

(fn `SpawnGunInHolster`
  (params (Parent :type "SceneComponent Object Reference"))
  (bind _returnvalue (`|SpawnActorFromClass` "/Game/VRGunToolkit/Blueprints/Weapons/Colt/BP_Colt1911_Arcade.BP_Colt1911_Arcade_C" (`KismetMathLibrary.MakeTransform` (0.0 0.0 0.0)) "AlwaysSpawn" "OverrideRootScale"))
  (`self.K2_AttachToComponent` _returnvalue Parent "None" "SnapToTarget" "SnapToTarget" "KeepWorld" true))

(fn `UserConstructionScript`
  (`parent.UserConstructionScript`))