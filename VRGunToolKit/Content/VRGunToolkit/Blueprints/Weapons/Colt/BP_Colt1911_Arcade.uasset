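; Arcade variant of the VR Colt 1911 pistol that starts with a magazine already in the gun.
; After the parent's BeginPlay, it spawns a Colt magazine, stores the reference and disables its physics and collision.
; It snaps the magazine mesh to the magazine's billboard and the magazine to the gun frame, then adjusts collision channel responses on both.
; All other behavior comes from the parent class.
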(event `self.ReceiveBeginPlay`
  ;[0.1227 0.3069 1] Automatically spawn a magazine in the gun
  (`parent.ReceiveBeginPlay`)
  (bind _returnvalue (`|SpawnActorFromClass` "/Game/VRGunToolkit/Blueprints/Weapons/Colt/BP_Colt1911_Magazine.BP_Colt1911_Magazine_C" (`KismetMathLibrary.MakeTransform` (0.0 0.0 0.0)) "Undefined" "OverrideRootScale" null null))
  (set `self.Magazine` _returnvalue)
  (bind _magazinemesh (`/Game/VRGunToolkit/Blueprints/BP_VRRealisticMagazine.MagazineMesh` _returnvalue))
  (`PrimitiveComponent.SetSimulatePhysics` _magazinemesh false)
  (`PrimitiveComponent.SetCollisionEnabled` _magazinemesh "NoCollision")
  (`PrimitiveComponent.SetCollisionEnabled` (`/Game/VRGunToolkit/Blueprints/BP_VRRealisticMagazine.MagazineCollision` _returnvalue) "NoCollision")
  (`SceneComponent.K2_AttachToComponent` _magazinemesh (`/Game/VRGunToolkit/Blueprints/BP_VRRealisticMagazine.Billboard` _returnvalue) "None" "SnapToTarget" "SnapToTarget" "KeepWorld" true)
  (`self.K2_AttachToComponent` _returnvalue (`self.Frame`) "None" "SnapToTarget" "SnapToTarget" "KeepWorld" true)
  (`PrimitiveComponent.SetCollisionResponseToChannel` (`/Game/VRGunToolkit/Blueprints/BP_VRRealisticMagazine.MagazineMesh` _returnvalue) "ECC_PhysicsBody" "ECR_Ignore")
  (`PrimitiveComponent.SetCollisionResponseToChannel` (`self.Frame`) "ECC_GameTraceChannel4" "ECR_Ignore"))

(fn `UserConstructionScript`
  (`parent.UserConstructionScript`))