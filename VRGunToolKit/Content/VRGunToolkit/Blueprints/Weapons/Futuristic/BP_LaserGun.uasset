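; BP_LaserGun is a futuristic VR Gun Toolkit weapon that flashes its glow whenever it fires.
; The construction script creates a dynamic material instance on the Frame and stores it as DynamicGunTexture.
; The Fire and FireLoop overrides call their parent logic and briefly raise the EmissiveIntensity parameter before resetting it, serving as a material animation example.
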(event `self.Fire`
  (bind _dynamicguntexture (`self.DynamicGunTexture`))
  ;[0.5571 1 0.696] Material Animation Example, the gun glows everytime we shoot
  (`MaterialInstanceDynamic.SetScalarParameterValue` _dynamicguntexture "EmissiveIntensity" 5.0)
  (`parent.Fire`)
  (`KismetSystemLibrary.Delay` 0.05)
  (`MaterialInstanceDynamic.SetScalarParameterValue` _dynamicguntexture "EmissiveIntensity" 1.0))

(event `self.FireLoop`
  (bind _dynamicguntexture (`self.DynamicGunTexture`))
  ;[0.5571 1 0.696] Material Animation Example, the gun glows everytime we shoot
  (`parent.FireLoop`)
  (`MaterialInstanceDynamic.SetScalarParameterValue` _dynamicguntexture "EmissiveIntensity" 5.0)
  (`KismetSystemLibrary.Delay` 0.05)
  (`MaterialInstanceDynamic.SetScalarParameterValue` _dynamicguntexture "EmissiveIntensity" 1.0))

(fn `UserConstructionScript`
  (`parent.UserConstructionScript`)
  (bind _returnvalue (`PrimitiveComponent.CreateDynamicMaterialInstance` (`self.Frame`) 0 "/Game/VRGunToolkit/Materials/Weapons/Futuristic/M_Light_ambient_occlusion_Mat.M_Light_ambient_occlusion_Mat"))
  (set `self.DynamicGunTexture` _returnvalue))